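; Moving platform that travels between a stored start and end position, optionally looping.
; After an initial delay, a custom event moves the mesh there and back with MoveComponentTo, pausing after each leg and calling itself while looping is on.
; The construction script uses self-resetting booleans as editor buttons to record the actor's location as either endpoint or snap the actor to one.
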(event `self.ReceiveBeginPlay`
  ;[1 1 1] Move Platform
  (`KismetSystemLibrary.Delay` (`self.Delay`))
  (`self.GoToLocationAndBack`))

(event `GoToLocationAndBack`
  (bind _returnvalue (`self.K2_GetActorRotation`))
  ;[1 1 1] Move Platform Back and Forth
  (`KismetSystemLibrary.MoveComponentTo` (`self.StaticMeshComponent`) (`self.EndPosition`) _returnvalue false false (`self.Speed`))
  (`KismetSystemLibrary.Delay` (`self.Delay`))
  (`KismetSystemLibrary.MoveComponentTo` (`self.StaticMeshComponent`) (`self.StartingPosition`) _returnvalue false false (`self.Speed`))
  (`KismetSystemLibrary.Delay` (`self.Delay`))
  (if (`self.PlatformIsLooping?`)
    (`self.GoToLocationAndBack`)))

(fn `UserConstructionScript`
  (bind _returnvalue (`self.K2_GetActorLocation`))
  (`|ExecutionSequence`
    (:`then_0`
      ;[1 1 1] Set Start and End Location of Platform
      (if (`self.SetStartPosition`)
        (set `self.StartingPosition` _returnvalue)
        (set `self.SetStartPosition` false)))
    (:`then_1`
      (if (`self.SetEndPosition`)
        (set `self.EndPosition` _returnvalue)
        (set `self.SetEndPosition` false)))
    (:`then_2`
      ;[1 1 1] Change Location
      (if (`self.GoToStartPosition`)
        (`self.K2_SetActorLocation` (`self.StartingPosition`))
        (set `self.GoToStartPosition` false)))
    (:`then_3`
      (if (`self.GoToEndPosition`)
        (`self.K2_SetActorLocation` (`self.EndPosition`))
        (set `self.GoToEndPosition` false)))))